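; AI sense component for BP_AiCharacter that tracks whether the player is visible and reports it to the GOAP controller.
; PawnSensing sightings are confirmed by a trace to the player's "visibility_querry" socket, which updates last location, broadcasts movement and holds a seeing flag for one sensing interval.
; Tick turns flag changes into gained/lost sight events, whose handlers recheck after PerceptionGap before sending an enemy visibility world event.
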(event `self.ReceiveBeginPlay`
  (bind _asbp_ai_character (cast `/Game/MyContent/Blueprints/AI/BP_AiCharacter` (`self.GetOwner`))
    (:`then`
      (bind _output_get (set `self.aiChar` _asbp_ai_character))
      (`/Engine/EditorBlueprintResources/StandardMacros.IsValid` _output_get
        (:`Is Valid`
          (bind _output_get_2 (set `self.PawnSense` (`/Game/MyContent/Blueprints/AI/BP_AiCharacter.PawnSensing` _output_get)))
          (add `PawnSensingComponent.OnSeePawn` _output_get_2 (delegate `OnSeePawn`))
          (add `self.OnGainedPlayerSight` (`|CreateDelegate` :!event `ProcessGainedPlayerSight`))
          (add `self.OnLostPlayerSight` (`|CreateDelegate` :!event `ProcessLostPlayerSight`)))
        (:`Is Not Valid`
          (`KismetSystemLibrary.PrintString` "Pawn Sense has not been init!" true true (struct :`G` 0.66 :`B` 1.0 :`A` 1.0) 12.0))))
    (:`CastFailed`
      (`KismetSystemLibrary.PrintString` "SenseManager owner is not aiCharacter"))))

(event `OnSeePawn`
  (params (Pawn :type "Pawn Object Reference"))
  ;[1 1 1] OnSeePawn
  (bind _asbp_third_person_character (cast `/Game/ThirdPerson/Blueprints/BP_ThirdPersonCharacter` Pawn))
  (bind _outhit (`KismetSystemLibrary.LineTraceSingle` (`Actor.K2_GetActorLocation` (`self.aiChar`)) (`SceneComponent.GetSocketLocation` (`Character.Mesh` _asbp_third_person_character) "visibility_querry") "TraceTypeQuery2"))
  (bind _asbp_third_person_character_2 (cast `/Game/ThirdPerson/Blueprints/BP_ThirdPersonCharacter` (`.HitActor` (`GameplayStatics.BreakHitResult` _outhit))))
  (bind _returnvalue (`Actor.K2_GetActorLocation` _asbp_third_person_character_2))
  (if (!= _returnvalue (`self.playerLastLocation`) :`ErrorTolerance` 1.0)
    (`self.OnPlayerMoved` _returnvalue (`self.playerLastLocation`)))
  (set `self.playerLastLocation` _returnvalue)
  (set `self.isSeeingPlayer` true)
  (`KismetSystemLibrary.Delay` (`PawnSensingComponent.SensingInterval` (`self.PawnSense`)))
  (set `self.isSeeingPlayer` false))

(event `self.ReceiveTick`
  (params (DeltaSeconds :type "Float (single-precision)"))
  ;[1 1 1] Tick
  (`/Game/MyContent/Blueprints/BPML_AComp.BoolTrigger` (`self.isSeeingPlayer`) true
    (:`TrueOut`
      (`self.OnGainedPlayerSight`))
    (:`FalseOut`
      (`self.OnLostPlayerSight`))))

(event `ProcessGainedPlayerSight`
  (`KismetSystemLibrary.Delay` (`self.PerceptionGap`))
  (if (`self.isSeeingPlayer`)
    (`/Game/MyContent/Blueprints/AI/BP_GoapController.ProcessWorldEvent` (`/Game/MyContent/Blueprints/AI/BP_AiCharacter.BP_GoapController` (`self.aiChar`)) (`|MakeMap` "AEnemyStatus" (`KismetMathLibrary.Conv_ByteToInt` (enumliteral `EAVEnemyStatus` "eVisible"))))
    (`KismetSystemLibrary.PrintString` "in sight!")))

(event `ProcessLostPlayerSight`
  (`KismetSystemLibrary.Delay` (`self.PerceptionGap`))
  (if (not (`self.isSeeingPlayer`))
    (`/Game/MyContent/Blueprints/AI/BP_GoapController.ProcessWorldEvent` (`/Game/MyContent/Blueprints/AI/BP_AiCharacter.BP_GoapController` (`self.aiChar`)) (`|MakeMap` "AEnemyStatus" (`KismetMathLibrary.Conv_ByteToInt` (enumliteral `EAVEnemyStatus` "eNonVisible"))))
    (`KismetSystemLibrary.PrintString` "in sight!")))