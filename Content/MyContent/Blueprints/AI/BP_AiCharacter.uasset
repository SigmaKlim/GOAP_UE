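; AI agent character driven by a GOAP controller, with a gun, health bar and actions for shooting, crouching, reloading and moving.
; Actions set state flags exposed through getters, with shooting adding focus and effects, and GoTo wrapping AIMoveTo in a DoOnce.
; Damage spawns blood, plays screams, updates the camera-facing bar and reports HP to the controller as a world event.
; Death ragdolls the mesh, disables movement and capsule collision, and reports goal failure.
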(event `self.ReceiveBeginPlay`
  (`|ExecutionSequence`
    (:`then_1`
      (add `self.OnTakePointDamage` (`|CreateDelegate` :!event `Receive Damage`)))
    (:`then_2`
      (set `/Game/MyContent/Blueprints/AI/BP_GoapController.aiChar` self (`self.BP_GoapController`)))))

(event `self.ReceiveTick`
  (params (DeltaSeconds :type "Float (single-precision)"))
  (bind _hpbar (`self.HpBar`))
  (if (`/Game/MyContent/Blueprints/AI/BP_GoapController.isAlive` (`self.BP_GoapController`))
    (`SceneComponent.K2_SetWorldRotation` _hpbar (`KismetMathLibrary.FindLookAtRotation` (`SceneComponent.K2_GetComponentLocation` _hpbar) (`SceneComponent.K2_GetComponentLocation` (`PlayerCameraManager.TransformComponent` (`GameplayStatics.GetPlayerCameraManager` 0)))) false false)))

(event `Shoot`
  (params (Target :type "Actor Object Reference"))
  (bind _gun (`self.Gun`))
  (bind _returnvalue (`SceneComponent.GetSocketLocation` _gun "b_gun_muzzleflash"))
  ;[1 1 1] Shoot
  (set `self.isAiming` true)
  (set `self.isShooting` true)
  (`AIController.K2_SetFocus` (`AIBlueprintHelperLibrary.GetAIController` self) Target)
  (`GameplayStatics.SpawnEmitterAttached` "/Game/MyContent/Assets/InfinityBladeEffects/Effects/FX_Monsters/FX_Monster_Gruntling/Master/P_BackPack_MuzzleFlash.P_BackPack_MuzzleFlash" (`self.Gun`) "b_gun_muzzleflash" _returnvalue (`SceneComponent.K2_GetComponentRotation` _gun) (0.1 0.1 0.1) "KeepWorldPosition" true "AutoRelease")
  (`GameplayStatics.PlaySoundAtLocation` "/Game/MyContent/Assets/Sound/shot.shot" _returnvalue (struct) 1.0 1.0 0.0 null null null null))

(event `StopShooting`
  ;[1 1 1] Shoot
  (`KismetSystemLibrary.RetriggerableDelay` 1.0)
  (`AIController.K2_ClearFocus` (`AIBlueprintHelperLibrary.GetAIController` self))
  (set `self.isAiming` false)
  (set `self.isShooting` false))

(event `Receive Damage`
  (params (DamagedActor :type "Actor Object Reference") (Damage :type "Float (single-precision)") (InstigatedBy :type "Controller Object Reference") (HitLocation :type "Vector Structure") (FHitComponent :type "PrimitiveComponent Object Reference") (BoneName :type Name) (ShotFromDirection :type "Vector Structure") (DamageType :type "DamageType Object Reference") (DamageCauser :type "Actor Object Reference"))
  (bind _screamplayer (`self.ScreamPlayer`))
  ;[1 1 1] Receive Damage
  (`GameplayStatics.SpawnEmitterAtLocation` "/Game/MyContent/Assets/Realistic_Starter_VFX_Pack_Vol2/Particles/Blood/P_Blood_Splat_Cone.P_Blood_Splat_Cone" HitLocation (`KismetMathLibrary.ComposeRotators` (`KismetMathLibrary.FindLookAtRotation` HitLocation ShotFromDirection) (struct :`Roll` 90.0)) (1.0 1.0 1.0) true "AutoRelease")
  (if (> (`self.hpLeft`) 0.0)
    (if (not (`AudioComponent.IsPlaying` _screamplayer))
      (`AudioComponent.Play` _screamplayer 0.0))
    (bind _output_get (set `self.hpLeft` (- (`self.hpLeft`) Damage)))
    (if (> _output_get 0.0)
      (`/Game/MyContent/Blueprints/UI/WBP_AgentHPBar.SetPercent` (cast `/Game/MyContent/Blueprints/UI/WBP_AgentHPBar` (`WidgetComponent.GetWidget` (`self.HpBar`)) :!pure true) (/ (`self.hpLeft`) 100.0))
      (else
        (`self.Die`)))
    (`/Game/MyContent/Blueprints/AI/BP_GoapController.ProcessWorldEvent` (`self.BP_GoapController`) (`|MakeMap` "AHpLeft" (`KismetMathLibrary.FTrunc` (`self.hpLeft`))))))

(event `StartCrouching`
  ;[1 1 1] Crouch
  (set `self.isCrouching` true))

(event `Die`
  ;[1 1 1] Die
  (`PrimitiveComponent.SetSimulatePhysics` (`self.Mesh`) true)
  (`CharacterMovementComponent.SetMovementMode` (`self.CharacterMovement`) "MOVE_None" 0)
  (`PrimitiveComponent.SetCollisionEnabled` (`self.CapsuleComponent`) "NoCollision")
  (set `/Game/MyContent/Blueprints/AI/BP_GoapController.isAlive` false (`self.BP_GoapController`))
  (`ActorComponent.K2_DestroyComponent` (`self.HpBar`))
  (`GoapController.ReportGoalFailed` (`self.BP_GoapController`)))

(event `StopCrouching`
  ;[1 1 1] Crouch
  (set `self.isCrouching` false))

(event `GoTo`
  (params (targetPoint :type "Vector Structure") (acceptanceRadius :type "Float (double-precision)"))
  ;[1 1 1] GoTo
  (`/Engine/EditorBlueprintResources/StandardMacros.DoOnce` false :!label _label
    (:`Completed`
      (set `self.isAtDestination` false)
      (`|AIMoveTo` self targetPoint null acceptanceRadius
        (:`OnSuccess`
          (set `self.isAtDestination` true)
          (goto _label :!via `Reset`))
        (:`OnFail`
          (`KismetSystemLibrary.PrintString` "GoToFailed")
          (goto _label :!via `Reset`))))))

(event `StopGoing`
  ;[1 1 1] GoTo
  (set `self.isAtDestination` false)
  (goto _label :!via `Reset`))

(event `Reload`
  (set `self.isReloading` true)
  (`KismetSystemLibrary.DelayUntilNextTick`)
  (set `self.isReloading` false))

(fn `GetIsAiming`
  (returns (isAiming :type Boolean))
  (return (`self.isAiming`)))

(fn `GetIsCrouching`
  (returns (isCrouching :type Boolean))
  (return (`self.isCrouching`)))

(fn `GetIsJumping`
  (returns (isJumping :type Boolean))
  (return false))

(fn `GetIsReloading`
  (returns (isReloading :type Boolean))
  (return (`self.isReloading`)))

(fn `GetIsShooting`
  (returns (isShooting :type Boolean))
  (return (`self.isShooting`)))

(fn `GetShotsPerSecond`
  (returns (shotsPerSecond :type "Float (double-precision)"))
  (return (`self.shotsPerSecond`)))

(fn `UserConstructionScript`
  (`|ExecutionSequence`
    (:`then_0`
      (`SceneComponent.K2_AttachToComponent` (`self.Gun`) (`self.Mesh`) "gun_socket" "KeepRelative" "KeepRelative" "KeepRelative" true))))