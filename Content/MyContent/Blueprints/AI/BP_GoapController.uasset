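; GOAP controller component that drives a BP_AiCharacter through crouch, stand, patrol, approach and shoot actions.
; Each Tick passes completion and rebuild flags to UpdateAi, then dispatches the returned action to a performer.
; Performers run every frame, using delay triggers for timing, and flag completion to advance the plan.
; ProcessWorldEvent overrides agent state, rebuilding the strategy on surprising effects or otherwise marking the action complete.
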(event `self.ReceiveBeginPlay`
  (`parent.ReceiveBeginPlay`)
  (bind _asbp_ai_character (cast `/Game/MyContent/Blueprints/AI/BP_AiCharacter` (`self.GetOwner`))
    (:`then`
      (bind _output_get (set `self.aiChar` _asbp_ai_character))
      (bind _bpc_sensemanager (`/Game/MyContent/Blueprints/AI/BP_AiCharacter.BPC_SenseManager` _output_get))
      (`/Engine/EditorBlueprintResources/StandardMacros.IsValid` _bpc_sensemanager
        (:`Is Valid`
          (set `self.senseManager` _bpc_sensemanager))
        (:`Is Not Valid`
          (`KismetSystemLibrary.PrintString` "Goap controller failed to reference SenseManager"))))
    (:`CastFailed`
      (`KismetSystemLibrary.PrintString` "GoapController owner is not aiCharacter"))))

(event `self.ReceiveTick`
  (params (DeltaSeconds :type "Float (single-precision)"))
  (bind (_actionname _effects) (`self.UpdateAi` (`self.wasPrevActionComplete`) (`self.mustRebuildStrategy`)))
  (set `self.mustRebuildStrategy` false)
  (set `self.wasPrevActionComplete` false)
  (`self.ChoosePerformer` _actionname _effects))

(event `PerformCrouch`
  ;[1 1 1] Crouch
  (`/Game/MyContent/Blueprints/BPML_AComp.DelayTrigger` 1.5 :!label _label
    (:`OutBefore`
      (`/Engine/EditorBlueprintResources/StandardMacros.DoOnce` false :!label _label_2
        (:`Completed`
          (`/Game/MyContent/Blueprints/AI/BP_AiCharacter.StartCrouching` (`self.aiChar`))
          (goto _label_3 :!via `Reset`))))
    (:`OutAfter`
      (set `self.wasPrevActionComplete` true)
      (goto _label_2 :!via `Reset`))))

(event `PerformStand`
  ;[1 1 1] Stand
  (`/Game/MyContent/Blueprints/BPML_AComp.DelayTrigger` 1.5 :!label _label_3
    (:`OutBefore`
      (`/Engine/EditorBlueprintResources/StandardMacros.DoOnce` false :!label _label_4
        (:`Completed`
          (`/Game/MyContent/Blueprints/AI/BP_AiCharacter.StopCrouching` (`self.aiChar`))
          (goto _label :!via `Reset`))))
    (:`OutAfter`
      (set `self.wasPrevActionComplete` true)
      (goto _label_4 :!via `Reset`))))

(event `PerformPatrol`
  (bind _aichar (`self.aiChar`))
  ;[1 1 1] Patrol
  (if (`/Game/MyContent/Blueprints/AI/BPC_SenseManager.isSeeingPlayer` (`/Game/MyContent/Blueprints/AI/BP_AiCharacter.BPC_SenseManager` (`self.aiChar`)))
    (`MovementComponent.StopMovementImmediately` (`Character.CharacterMovement` _aichar))
    (`/Game/MyContent/Blueprints/AI/BP_AiCharacter.StopGoing` _aichar)
    (set `self.wasPrevActionComplete` true)
    (elif (`/Game/MyContent/Blueprints/AI/BP_AiCharacter.isAtDestination` _aichar)
      (bind _point (`self.SelectPatrolPoint`))
      (`/Game/MyContent/Blueprints/AI/BP_AiCharacter.GoTo` _aichar _point 5.0))))

(event `PerformApproach`
  (bind _aichar (`self.aiChar`))
  ;[1 1 1] Approach
  (`/Game/MyContent/Blueprints/AI/BP_AiCharacter.GoTo` (`self.aiChar`) (`GameplayStatics.GetPlayerCharacter` 0) 500.0)
  (bind _output_get (set `self.wasPrevActionComplete` (`/Game/MyContent/Blueprints/AI/BP_AiCharacter.isAtDestination` (`self.aiChar`))))
  (if _output_get
    (`MovementComponent.StopMovementImmediately` (`Character.CharacterMovement` _aichar))
    (`/Game/MyContent/Blueprints/AI/BP_AiCharacter.StopGoing` _aichar)))

(event `PerformShoot`
  (bind _aichar (`self.aiChar`))
  (bind _aichar_2 (`self.aiChar`))
  (`Actor.K2_SetActorRotation` _aichar_2 (`KismetMathLibrary.RInterpTo` (`Actor.K2_GetActorRotation` _aichar_2) (`KismetMathLibrary.FindRelativeLookAtRotation` (`Actor.GetTransform` _aichar_2) (`Actor.K2_GetActorLocation` (`GameplayStatics.GetPlayerCharacter` 0))) (`GameplayStatics.GetWorldDeltaSeconds`) 10.0) true)
  (`/Game/MyContent/Blueprints/BPML_AComp.DelayTrigger` (/ 1.0 (`/Game/MyContent/Blueprints/AI/BP_AiCharacter.shotsPerSecond` _aichar)) :!label _label_5
    (:`OutAfter`
      (`/Game/MyContent/Blueprints/AI/BP_AiCharacter.Shoot` _aichar)
      (set `self.wasPrevActionComplete` true)
      (goto _label_5 :!via `Reset`))))

(fn `ChoosePerformer`
  (params (ActionName :type String) (Effects :type "Map of String to Integer"))
  (switch `string` ActionName
    (:`Default`
      (`KismetSystemLibrary.PrintString` (`KismetStringLibrary.Concat_StrStr` "Can't choose performer for action:" ActionName)))
    (:`AcCrouch`
      ;[1 1 1] Performers, called each frame!!!
      (`self.PerformCrouch`)
      (`KismetSystemLibrary.PrintString` "Crouch"))
    (:`AcStand`
      (`self.PerformStand`)
      (`KismetSystemLibrary.PrintString` "Stand"))
    (:`AcPatrol`
      (`self.PerformPatrol`))
    (:`AcApproach`
      (`self.PerformApproach`))
    (:`AcShoot`
      (`self.PerformShoot`))))

(fn `ProcessWorldEvent`
  (params (effects :type "Map of String to Integer"))
  (if (`self.IsSurprised` effects)
    (set `self.mustRebuildStrategy` true)
    (else
      (set `self.wasPrevActionComplete` true)))
  (`self.OverrideAgentState` effects))

(fn `RequestStrategyRebuild`
  (set `self.mustRebuildStrategy` true))

(fn `SelectPatrolPoint`
  (returns (Point :type "TargetPoint Object Reference"))
  (bind _patrolindex (`self.patrolIndex`))
  (bind _aichar (`self.aiChar`))
  (`/Engine/EditorBlueprintResources/StandardMacros.IncrementInt` _patrolindex
    (:`  `
      (bind _output_get (set `self.patrolIndex` (`KismetMathLibrary.FTrunc` (`KismetMathLibrary.FMod` (`KismetMathLibrary.Conv_IntToDouble` _patrolindex) (`KismetMathLibrary.Conv_IntToDouble` (`KismetArrayLibrary.Array_Length` (`/Game/MyContent/Blueprints/AI/BP_AiCharacter.PatrolPointIndices` (`self.aiChar`))))))))
      (return (`|GetArrayItem` (`/Game/MyContent/Blueprints/AI/BP_AiCharacter.PatrolPoints` _aichar) (`|GetArrayItem` (`/Game/MyContent/Blueprints/AI/BP_AiCharacter.PatrolPointIndices` _aichar) _output_get))))))