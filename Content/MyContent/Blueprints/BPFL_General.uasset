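; General-purpose Blueprint function library with a Wrap helper that cycles an integer into a range from zero to an upper bound.
; Values already inside the range, exclusive of the bound, pass through unchanged.
; Otherwise it takes the remainder of the absolute value divided by the bound, and nested selects return either that remainder or the bound minus it for negative wrapping.
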(fn `Wrap`
  (params (AttemptedValue :type Integer) (UpperBound :type Integer))
  (returns (ResultValue :type Integer))
  (bind _remainder (`KismetMathLibrary.FMod` (`KismetMathLibrary.Conv_IntToDouble` (`KismetMathLibrary.Abs_Int` AttemptedValue)) (`KismetMathLibrary.Conv_IntToDouble` UpperBound)))
  (return (`KismetMathLibrary.SelectInt` AttemptedValue (`KismetMathLibrary.SelectInt` (- UpperBound _remainder) (`KismetMathLibrary.FTrunc` _remainder) (< 0 0)) (`KismetMathLibrary.InRange_IntInt` AttemptedValue 0 UpperBound true false))))