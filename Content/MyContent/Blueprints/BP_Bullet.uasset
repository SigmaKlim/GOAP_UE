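; Bullet projectile actor that shows a surface-specific impact effect when its collider overlaps a tagged actor.
; Overlaps with Prop or Enemy tags swap the initially inactive particle system to concrete or blood, activate it, and zero the projectile velocity.
; The bullet then destroys itself after a short delay, or earlier if an overlap ends once the hit flag is set.
; Other actors are ignored, and no damage is applied here.
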(event `self.ReceiveBeginPlay`
  (`ActorComponent.Deactivate` (`self.ParticleSystem1`)))

(event `self.Collider.OnComponentBeginOverlap`
  (params (OverlappedComponent :type "PrimitiveComponent Object Reference") (OtherActor :type "Actor Object Reference") (OtherComp :type "PrimitiveComponent Object Reference") (OtherBodyIndex :type Integer) (bFromSweep :type Boolean) (SweepResult :type "HitResult Structure (by ref)"))
  (bind _particlesystem1 (`self.ParticleSystem1`))
  (if (`self.ActorHasTag` OtherActor "Prop")
    (`ParticleSystemComponent.SetTemplate` _particlesystem1 "/Game/MyContent/Assets/Realistic_Starter_VFX_Pack_Vol2/Particles/Hit/P_Concrete.P_Concrete")
    (`ActorComponent.Activate` _particlesystem1 false :!label _label)
    (set `self.hasHit` true)
    (set `MovementComponent.Velocity` (0.0 0.0 0.0) (`self.ProjectileMovement`))
    (`KismetSystemLibrary.Delay` 2.0)
    (`self.K2_DestroyActor`)
    (elif (`self.ActorHasTag` OtherActor "Enemy")
      (`ParticleSystemComponent.SetTemplate` _particlesystem1 "/Game/MyContent/Assets/Realistic_Starter_VFX_Pack_Vol2/Particles/Blood/P_Blood_Splat_Cone.P_Blood_Splat_Cone")
      (goto _label))))

(event `self.Collider.OnComponentEndOverlap`
  (params (OverlappedComponent :type "PrimitiveComponent Object Reference") (OtherActor :type "Actor Object Reference") (OtherComp :type "PrimitiveComponent Object Reference") (OtherBodyIndex :type Integer))
  (if (`self.hasHit`)
    (`self.K2_DestroyActor`)))

(fn `UserConstructionScript`)