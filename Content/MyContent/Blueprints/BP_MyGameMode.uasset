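; Game mode that adds a debug observer for GOAP-driven AI agents, gathering every BP_AiCharacter at BeginPlay and keeping the player controller ticking during pause.
; Debug keys toggle pause, toggle observation while paused, and cycle through agents.
; StartObserving moves the view to the agent and fills WBP_ObservationWindow with its controller's strategy, plan and state.
; StopOberving restores the player view and game input, also on unpause.
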(event EventBeginPlay
  (bind _returnvalue (Game|GetPlayerController 0))
  (Input|EnableInput _returnvalue)
  (bind _outactors (Actor|GetAllActorsOfClass "/Game/MyContent/Blueprints/AI/BP_AiCharacter.BP_AiCharacter_C"))
  (Variables|Observation|SetaiAgents _outactors)
  (Variables|/Script/Engine.PlayerController|SetbShouldPerformFullTickWhenPaused _returnvalue true))

(event Input|KeyboardEvents|DebugKeyRight
  (params (Key :type Key%20Structure :default "None") (ActionValue :type Input%20Action%20Value%20Structure))
  ;[1 1 1] Scroll observants
  (:Pressed
    (if (Variables|Observation|GetisObservingAgents)
      (Variables|Observation|SetobservedAgentIndex (CallFunction|Wrap (+ (Variables|Observation|GetobservedAgentIndex) -1) (Utilities|Array|Length (Variables|Observation|GetaiAgents))))
      (CallFunction|StartObserving))))

(event Input|KeyboardEvents|DebugKeyO
  (params (Key :type Key%20Structure :default "None") (ActionValue :type Input%20Action%20Value%20Structure))
  ;[1 1 1] Enable observation
  (:Pressed
    (if (Game|IsGamePaused)
      (Utilities|FlowControl|FlipFlop
        (:A
          (CallFunction|StartObserving))
        (:B
          (CallFunction|StopOberving))))))

(event Input|KeyboardEvents|DebugKeyLeft
  (params (Key :type Key%20Structure :default "None") (ActionValue :type Input%20Action%20Value%20Structure))
  ;[1 1 1] Scroll observants
  (:Pressed
    (if (Variables|Observation|GetisObservingAgents)
      (Variables|Observation|SetobservedAgentIndex (CallFunction|Wrap (+ (Variables|Observation|GetobservedAgentIndex) 1) (Utilities|Array|Length (Variables|Observation|GetaiAgents))))
      (CallFunction|StartObserving))))

(event Input|KeyboardEvents|DebugKeyP
  (params (Key :type Key%20Structure :default "None") (ActionValue :type Input%20Action%20Value%20Structure))
  ;[1 1 1] Pause On/ Off
  (:Pressed
    (Utilities|FlowControl|FlipFlop
      (:A
        (Game|SetGamePaused true))
      (:B
        (Game|SetGamePaused false)
        ;[1 1 1] Enable observation
        (CallFunction|StopOberving)))))

(fn ConstructionScript)

(fn StartObserving
  (bind _returnvalue (Game|GetPlayerController 0))
  (bind _aiagents (Variables|Observation|GetaiAgents))
  (bind _observedagentindex (Variables|Observation|GetobservedAgentIndex))
  (bind _output (Utilities|Array|Get(acopy) _aiagents _observedagentindex))
  (Variables|/Script/Engine.PlayerController|SetbShowMouseCursor _returnvalue true)
  (Input|SetInputModeUIOnly _returnvalue 0 "DoNotLock" false)
  (Utilities|IsValid (Variables|Observation|GetobservationWidget)
    (:Is%20Valid
      (Widget|RemovefromParent (Variables|Observation|GetobservationWidget)))
    (:Is%20Not%20Valid
      _))
  (Variables|Observation|SetisObservingAgents true)
  (LocalVariables|SetobservedController (Variables|/Game/MyContent/Blueprints/AI/BP_AiCharacter.BP_AiCharacter_C|GetBP_GoapController _output))
  (Game|Player|SetViewTargetwithBlend (Game|GetPlayerController 0) _output 0.0 "VTBlend_Linear" 0.0 false)
  (bind _returnvalue_2 (UserInterface|CreateWidget "/Game/MyContent/Blueprints/UI/WBP_ObservationWindow.WBP_ObservationWindow_C"))
  (bind _output_get (Variables|Observation|SetobservationWidget _returnvalue_2))
  (UserInterface|Viewport|AddtoViewport _output_get 0)
  (Default|SetId _returnvalue_2 (Variables|Observation|GetobservedAgentIndex))
  (for (_array_element _array_index) (Class|GoapController|GetCurrentStrategy (LocalVariables|GetobservedController))
    (Default|AddGoaltoStrategy (Variables|Observation|GetobservationWidget) _array_index (Utilities|Array|Get(acopy) (Variables|Default|GetGoalNames) _array_element) (== _array_index (Class|GoapController|GetCurrentGoalIndex (LocalVariables|GetobservedController)))))
  (for (_array_element_2 _array_index_2) (Class|GoapController|GetCurrentPlan (LocalVariables|GetobservedController))
    (Default|AddActiontoPlan (Variables|Observation|GetobservationWidget) _array_index_2 (Utilities|Array|Get(acopy) (Variables|Default|GetActionNames) _array_element_2) (== _array_index_2 (Class|GoapController|GetCurrentActionIndex (LocalVariables|GetobservedController)))))
  (for (_array_element_3 _array_index_3) (Class|GoapController|GetCurrentState (LocalVariables|GetobservedController))
    (Default|AddAttributeValue (Variables|Observation|GetobservationWidget) _array_index_3 (Utilities|Array|Get(acopy) (Variables|Default|GetAttributeNames) _array_element_3) (Class|GoapController|GetAttributeValueString (LocalVariables|GetobservedController) _array_index_3 _array_element_3))))

(fn StopOberving
  (bind _returnvalue (Game|GetPlayerController 0))
  (Variables|/Script/Engine.PlayerController|SetbShowMouseCursor _returnvalue true)
  (Input|SetInputModeGameOnly _returnvalue false)
  (Widget|RemovefromParent (Variables|Observation|GetobservationWidget))
  (Game|Player|SetViewTargetwithBlend (Game|GetPlayerController 0) (Game|GetPlayerCharacter 0) 0.0 "VTBlend_Linear" 0.0 false)
  (Variables|Observation|SetisObservingAgents false))