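; BP_InterestPoint is an interest point actor that reports itself as really interesting only while it is hidden from the player.
; IsReallyInteresting ignores its agent argument and returns the inverse of IsVisibleToPlayer.
; IsVisibleToPlayer line-traces on the Visibility channel from the Cylinder component to the player character's visibility_querry mesh socket, counting only a blocking hit on that character as visible.
; It has no active event or construction logic.
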(fn `IsReallyInteresting`
  (params (agentPtr :type "Character Object Reference"))
  (returns (ReturnValue :type Boolean))
  (return (not (`self.IsVisibleToPlayer`))))

(fn `IsVisibleToPlayer`
  (returns (ReturnValue :type Boolean))
  (bind _outhit (`KismetSystemLibrary.LineTraceSingle` (`SceneComponent.K2_GetComponentLocation` (`self.Cylinder`)) (`SceneComponent.GetSocketLocation` (`Character.Mesh` (`GameplayStatics.GetPlayerCharacter` 0)) "visibility_querry") "TraceTypeQuery1"))
  (bind (_bblockinghit _binitialoverlap _time _distance _location _impactpoint _normal _impactnormal _physmat _hitactor) (`GameplayStatics.BreakHitResult` _outhit))
  (return (and _bblockinghit (== _hitactor (`GameplayStatics.GetPlayerCharacter` 0)))))

(fn `UserConstructionScript`)