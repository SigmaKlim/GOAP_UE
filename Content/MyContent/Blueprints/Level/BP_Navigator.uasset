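; BP_Navigator is a level helper Blueprint that measures navigation distance between two actors.
; GetDistance runs a GetPathLength query between their locations and returns the path length when it succeeds.
; On failure it falls back to GetMaxDistance, which is four times the straight-line distance between the Marker1 and Marker2 components.
; It has no active event or construction logic.
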(fn `GetDistance`
  (params (from :type "InterestPoint Object Reference") (to :type "InterestPoint Object Reference"))
  (returns (ReturnValue :type "Float (single-precision)"))
  (bind (_pathlength _returnvalue) (`NavigationSystemV1.GetPathLength` (`self.K2_GetActorLocation` from) (`self.K2_GetActorLocation` to) null null))
  (return (`KismetMathLibrary.SelectFloat` _pathlength (`self.GetMaxDistance`) (`|EnumEquality` _returnvalue "Success"))))

(fn `GetMaxDistance`
  (returns (ReturnValue :type "Float (single-precision)"))
  (return (* (`KismetMathLibrary.Vector_Distance` (`SceneComponent.K2_GetComponentLocation` (`self.Marker1`)) (`SceneComponent.K2_GetComponentLocation` (`self.Marker2`))) 4.0)))

(fn `UserConstructionScript`)